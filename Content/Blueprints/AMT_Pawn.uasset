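; Player pawn for a measuring tool, with a free-fly camera that has adjustable speed and RMB-gated look and FOV zoom.
; It creates the menu widget, whose mode and type decide whether left click makes lines or 2D/3D shapes on the latest Measure actor.
; Custom events spawn and destroy measures, and a looping timer line-traces from the camera to position their spheres.
; The action button ends creation.
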(event `Spawn single measure`
  (params (`1st` :type Boolean) (Location :type "Vector Structure"))
  (bind _returnvalue (`|SpawnActorFromClass` "/Game/Blueprints/Measure.Measure_C" (`KismetMathLibrary.MakeTransform` Location (struct) (0.1 0.1 0.1)) "Undefined" "OverrideRootScale" null null))
  (bind _output_get (set `self.Last Measure ref` _returnvalue))
  (if (not `1st`)
    (`/Game/Blueprints/Measure.Create multiple lines` _output_get)))

(event `self.ReceiveBeginPlay`
  (`self.Draw HUD`))

(event `Destroy measure`
  (`/Engine/EditorBlueprintResources/StandardMacros.IsValid` (`self.Last Measure ref`)
    (:`Is Valid`
      (`self.K2_DestroyActor` (`self.Last Measure ref`)))))

(event `InputAction|LMB`
  (params (Key :type "Key Structure"))
  (bind _last_measure_ref (`self.Last Measure ref`))
  ;[1 1 1] LMB
  (:`Pressed`
    (switch `/Game/Enum/Menu_Modes` (`/Game/Widgets/Menu_UMG.Menu mode` (`self.Menu ref`))
      (:`NewEnumerator1`
        (switch `/Game/Enum/Create_Type` (`/Game/Widgets/Menu_UMG.Type` (`self.Menu ref`))
          (:`NewEnumerator0`
            (`/Game/Blueprints/Measure.Create single line` _last_measure_ref))
          (:`NewEnumerator1`
            (`/Game/Blueprints/Measure.Create multiple lines` _last_measure_ref))
          (:`NewEnumerator2`
            (`/Game/Blueprints/Measure.Create 2D Shape` (`self.Last Measure ref`) (`/Game/Widgets/Menu_UMG.2D Shape` (`self.Menu ref`))))
          (:`NewEnumerator3`
            (`/Game/Blueprints/Measure.Create 3D Shape` (`self.Last Measure ref`) (`/Game/Widgets/Menu_UMG.3D Shape` (`self.Menu ref`)))))))))

(event `InputAction|RMB`
  (params (Key :type "Key Structure"))
  ;[0.1714 0.1771 0.07809] set RMB bool
  (:`Pressed`
    (set `self.RMB` true))
  (:`Released`
    (set `self.RMB` false)))

(event `InputAxis|Move on X`
  (params (AxisValue :type "Float (single-precision)"))
  ;[0.05729 0.05504 0.02071] Player movement
  (`SceneComponent.K2_AddWorldOffset` (`self.Camera`) (* (`KismetMathLibrary.GetForwardVector` (`SceneComponent.K2_GetComponentRotation` (`self.Camera`))) (* AxisValue (`self.Moving Speed`))) false true))

(event `Draw HUD`
  ;[0.07733 0.09896 0.02393] Draw HUD
  (bind _returnvalue (`|CreateWidget` "/Game/Widgets/Menu_UMG.Menu_UMG_C" (`GameplayStatics.GetPlayerController` 0)))
  (bind _output_get (set `self.Menu ref` _returnvalue))
  (`UserWidget.AddToViewport` _output_get 0))

(event `InputAxis|Move on Y`
  (params (AxisValue :type "Float (single-precision)"))
  ;[0.05729 0.05504 0.02071] Player movement
  (`SceneComponent.K2_AddWorldOffset` (`self.Camera`) (* (`KismetMathLibrary.GetRightVector` (`SceneComponent.K2_GetComponentRotation` (`self.Camera`))) (* AxisValue (`self.Moving Speed`))) false true))

(event `InputAxis|Move on Z`
  (params (AxisValue :type "Float (single-precision)"))
  ;[0.05729 0.05504 0.02071] Player movement
  (`SceneComponent.K2_AddWorldOffset` (`self.Camera`) (`KismetMathLibrary.MakeVector` 0.0 0.0 (* AxisValue (`self.Moving Speed`))) false true))

(event `InputAxis|Look on Y`
  (params (AxisValue :type "Float (single-precision)"))
  ;[0.05729 0.05504 0.02071] Player movement
  (if (`self.RMB`)
    (`SceneComponent.K2_AddRelativeRotation` (`self.Camera`) (`KismetMathLibrary.MakeRotator` 0.0 AxisValue) false false)))

(event `InputAxis|Look on X`
  (params (AxisValue :type "Float (single-precision)"))
  ;[0.05729 0.05504 0.02071] Player movement
  (if (`self.RMB`)
    (`SceneComponent.K2_AddRelativeRotation` (`self.Camera`) (`KismetMathLibrary.MakeRotator` 0.0 0.0 AxisValue) false false)))

(event `InputAction|Actor speed +`
  (params (Key :type "Key Structure"))
  ;[0.05729 0.05504 0.02071] Player movement
  (:`Pressed`
    (if (>= (`self.Moving Speed`) 10.0)
      (set `self.Moving Speed` 10.0)
      (else
        (set `self.Moving Speed` (+ (`self.Moving Speed`) 1.0))))))

(event `InputAction|Action button`
  (params (Key :type "Key Structure"))
  (bind _last_measure_ref (`self.Last Measure ref`))
  ;[1 1 1] e
  (:`Pressed`
    (`/Engine/EditorBlueprintResources/StandardMacros.IsValid` _last_measure_ref
      (:`Is Valid`
        (if (`/Game/Blueprints/Measure.IsCreating` _last_measure_ref)
          (`/Game/Blueprints/Measure.Stop creating` (`self.Last Measure ref`)))))))

(event `InputAction|Actor speed -`
  (params (Key :type "Key Structure"))
  ;[0.05729 0.05504 0.02071] Player movement
  (:`Pressed`
    (if (<= (`self.Moving Speed`) 1.0)
      (set `self.Moving Speed` 1.0)
      (else
        (set `self.Moving Speed` (- (`self.Moving Speed`) 1.0))))))

(event `Add FOV STOP`
  ;[0.05729 0.05504 0.02071] Player movement
  (`KismetSystemLibrary.K2_ClearAndInvalidateTimerHandle` (stale `Add FOV` _returnvalue)))

(event `Add FOV`
  (bind _camera (`self.Camera`))
  (bind _fieldofview (`CameraComponent.FieldOfView` _camera))
  ;[0.05729 0.05504 0.02071] Player movement
  (bind _returnvalue (`KismetSystemLibrary.K2_SetTimerDelegate` (delegate `Add FOV`) 0.01 true))
  (if (<= _fieldofview 90.0)
    (set `CameraComponent.FieldOfView` (+ _fieldofview 1.0) _camera)
    (else
      (set `CameraComponent.FieldOfView` 90.0 _camera))))

(event `InputAction|FOV +`
  (params (Key :type "Key Structure"))
  ;[0.05729 0.05504 0.02071] Player movement
  (:`Pressed`
    (if (`self.RMB`)
      (`self.Add FOV`)))
  (:`Released`
    (`self.Add FOV STOP`)))

(event `Subtract FOV STOP`
  ;[0.05729 0.05504 0.02071] Player movement
  (`KismetSystemLibrary.K2_ClearAndInvalidateTimerHandle` (stale `Subtract FOV` _returnvalue)))

(event `Subtract FOV`
  (bind _camera (`self.Camera`))
  (bind _fieldofview (`CameraComponent.FieldOfView` _camera))
  ;[0.05729 0.05504 0.02071] Player movement
  (bind _returnvalue (`KismetSystemLibrary.K2_SetTimerDelegate` (delegate `Subtract FOV`) 0.01 true))
  (if (>= _fieldofview 5.0)
    (set `CameraComponent.FieldOfView` (- _fieldofview 1.0) _camera)
    (else
      (set `CameraComponent.FieldOfView` 5.0 _camera))))

(event `InputAction|FOV -`
  (params (Key :type "Key Structure"))
  ;[0.05729 0.05504 0.02071] Player movement
  (:`Pressed`
    (if (`self.RMB`)
      (`self.Subtract FOV`)))
  (:`Released`
    (`self.Subtract FOV STOP`)))

(event `Create mode update STOP`
  ;[1 1 1] Create mode: update spheres
  (`KismetSystemLibrary.K2_ClearAndInvalidateTimerHandle` (stale `Create mode update` _returnvalue_2)))

(event `Create mode update`
  (bind _camera (`self.Camera`))
  (bind _last_measure_ref (`self.Last Measure ref`))
  (bind _camera_2 (`self.Camera`))
  (bind _returnvalue (`SceneComponent.K2_GetComponentLocation` _camera_2))
  ;[1 1 1] Create mode: update spheres
  (bind _returnvalue_2 (`KismetSystemLibrary.K2_SetTimerDelegate` (delegate `Create mode update`) 0.01 true))
  (bind _outhit (`KismetSystemLibrary.LineTraceSingle` :`Start` _returnvalue :`End` (+ _returnvalue (* (`SceneComponent.GetForwardVector` _camera_2) (`KismetMathLibrary.SelectFloat` 999999.0 (`self.Trace length`) (`/Game/Widgets/Menu_UMG.Infinite distance` (`self.Menu ref`))))) :`TraceChannel` "TraceTypeQuery1" :`DrawTime` 1.0))
  (if (`GameplayStatics.BreakHitResult` _outhit)
    (set `self.Trace End Location` (`.Location` (`GameplayStatics.BreakHitResult` _outhit)))
    (else
      (set `self.Trace End Location` (+ (`SceneComponent.K2_GetComponentLocation` _camera) (* (`SceneComponent.GetForwardVector` _camera) (`KismetMathLibrary.SelectFloat` 999999.0 (`self.Trace length`) (`/Game/Widgets/Menu_UMG.Infinite distance` (`self.Menu ref`))))))))
  (`/Engine/EditorBlueprintResources/StandardMacros.IsValid` _last_measure_ref
    (:`Is Valid`
      (`/Game/Blueprints/Measure.Update Basic Spheres Location` _last_measure_ref (`self.Trace End Location`)))))

(fn `UserConstructionScript`)